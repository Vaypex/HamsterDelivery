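; Gameplay player controller that manages the local player's match UI and pawn input.
; On local BeginPlay it clears widgets and builds the main Interface, whose player list is cleared and filled through controller events.
; Other events show countdown and winner widgets and enable or disable pawn input for round start and end freezes.
; The F key calls Countdown directly on Gameplay_GameMode.
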(event `self.ReceiveBeginPlay`
  ;[1 1 1] Begin Play
  (if (`self.IsLocalController`)
    (`WidgetLayoutLibrary.RemoveAllWidgets`)
    (`self.Setup_UI`)))

(event `Setup_UI`
  ;[1 1 1] Interface
  (bind _returnvalue (`|CreateWidget` "/Game/Blueprints/UI/Interface.Interface_C" (`GameplayStatics.GetPlayerController` 0)))
  (bind _output_get (set `self.Interface` _returnvalue))
  (`UserWidget.AddToViewport` _output_get 0)
  (`self.AddPlayerToWindow` ""))

(event `UpdateBoxesInCharacter`)

(event `ShowWinnerWidget`
  (params (Won :type Boolean))
  (`WidgetLayoutLibrary.RemoveAllWidgets`)
  (bind _returnvalue (`|CreateWidget` "/Game/Widgets/W_Winner.W_Winner_C" null Won))
  (`UserWidget.AddToViewport` _returnvalue 0))

(event `ShowCountdown`
  ;[1 1 1] Таймер в начале игры
  (bind _returnvalue (`|CreateWidget` "/Game/Widgets/W_CountDown.W_CountDown_C"))
  (`UserWidget.AddToViewport` _returnvalue 0))

(event `Key|F`
  (params (Key :type "Key Structure"))
  (:`Pressed`
    (bind _asgameplay_game_mode (cast `/Game/Blueprints/Gameplay_GameMode` (`GameplayStatics.GetGameMode`)))
    (`/Game/Blueprints/Gameplay_GameMode.Countdown` _asgameplay_game_mode)))

(event `UnfreezePlayers`
  ;[1 1 1] Таймер в начале игры
  (`self.EnableInput` (`self.K2_GetPawn`) self))

(event `EndGameFreeze`
  (`self.DisableInput` (`self.K2_GetPawn`) self))

(event `ClearPlayerLust`
  (`/Game/Blueprints/UI/Interface.ClearPlayerList` (`self.Interface`)))

(event `AddPlayerToWindow`
  (params (PlayerName :type Text) (BoxesInPlayer :type Integer) (PlayerPlace :type Integer) (PlayerImage :type "Texture2D Object Reference"))
  (`/Game/Blueprints/UI/Interface.AddPlayerToList` (`self.Interface`) PlayerName BoxesInPlayer PlayerPlace PlayerImage))

(fn `GameplayPCRef`
  (returns (`Player Controller` :type "/Game/Blueprints/Gameplay_PlayerController Object Reference"))
  (return null))

(fn `UserConstructionScript`)