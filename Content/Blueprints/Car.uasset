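; Car actor that rides along a spline and lets Hamster characters hitch onto either side.
; On BeginPlay a server-named start event plays a timeline, whose track supplies spline time to move and rotate the skeletal mesh.
; Left and right box overlaps snap the Hamster to the matching mesh socket through a server-named grab event, and ending the overlap detaches it.
; The front box overlap is an empty stub.
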(event `Server_StartCar`
  ;[1 1 1] Передвижение
  (`self.GoCar`))

(event `GoCar`
  (bind _spline (`self.Spline`))
  ;[1 1 1] Передвижение
  (bind (_direction _newtrack_0) (`Timeline|Timeline_0`)
    (:`Update`
      (`SceneComponent.K2_SetWorldLocationAndRotation` (`self.SkeletalMesh`) (`SplineComponent.GetLocationAtTime` _spline _newtrack_0 "World" false) (`SplineComponent.GetRotationAtTime` _spline _newtrack_0 "World" false) false false))))

(event `self.ReceiveBeginPlay`
  ;[1 1 1] Передвижение
  (`self.Server_StartCar`))

(event `self.RightBox.OnComponentBeginOverlap`
  (params (OverlappedComponent :type "PrimitiveComponent Object Reference") (OtherActor :type "Actor Object Reference") (OtherComp :type "PrimitiveComponent Object Reference") (OtherBodyIndex :type Integer) (bFromSweep :type Boolean) (SweepResult :type "HitResult Structure (by ref)"))
  ;[1 1 1] Зацеп
  (bind _ashamster (cast `/Game/Character/Humster/Hamster` OtherActor))
  (bind _output_get (set `self.Humster` _ashamster))
  (`self.Server_CarGrab` _output_get "RightSoket"))

(event `self.LeftBox.OnComponentBeginOverlap`
  (params (OverlappedComponent :type "PrimitiveComponent Object Reference") (OtherActor :type "Actor Object Reference") (OtherComp :type "PrimitiveComponent Object Reference") (OtherBodyIndex :type Integer) (bFromSweep :type Boolean) (SweepResult :type "HitResult Structure (by ref)"))
  ;[1 1 1] Зацеп
  (bind _ashamster (cast `/Game/Character/Humster/Hamster` OtherActor))
  (bind _output_get (set `self.Humster` _ashamster))
  (`self.Server_CarGrab` _output_get "LeftSoket"))

(event `self.RightBox.OnComponentEndOverlap`
  (params (OverlappedComponent :type "PrimitiveComponent Object Reference") (OtherActor :type "Actor Object Reference") (OtherComp :type "PrimitiveComponent Object Reference") (OtherBodyIndex :type Integer))
  ;[1 1 1] Зацеп
  (bind _ashamster (cast `/Game/Character/Humster/Hamster` OtherActor))
  (`self.UnGrab` _ashamster))

(event `self.LeftBox.OnComponentEndOverlap`
  (params (OverlappedComponent :type "PrimitiveComponent Object Reference") (OtherActor :type "Actor Object Reference") (OtherComp :type "PrimitiveComponent Object Reference") (OtherBodyIndex :type Integer))
  ;[1 1 1] Зацеп
  (bind _ashamster (cast `/Game/Character/Humster/Hamster` OtherActor))
  (`self.UnGrab` _ashamster))

(event `Server_CarGrab`
  (params (Hunster :type "Actor Object Reference") (Side :type Name))
  ;[1 1 1] Зацеп
  (bind _ashamster (cast `/Game/Character/Humster/Hamster` Hunster))
  (`self.K2_AttachToComponent` _ashamster (`self.SkeletalMesh`) Side "SnapToTarget" "SnapToTarget" "KeepWorld" false))

(event `UnGrab`
  (params (NewParam :type "Actor Object Reference"))
  ;[1 1 1] Зацеп
  (bind _ashamster (cast `/Game/Character/Humster/Hamster` NewParam))
  (`self.K2_DetachFromActor` _ashamster "KeepWorld" "KeepWorld" "KeepWorld"))

(event `self.FrontBox.OnComponentBeginOverlap`
  (params (OverlappedComponent :type "PrimitiveComponent Object Reference") (OtherActor :type "Actor Object Reference") (OtherComp :type "PrimitiveComponent Object Reference") (OtherBodyIndex :type Integer) (bFromSweep :type Boolean) (SweepResult :type "HitResult Structure (by ref)")))

(fn `UserConstructionScript`)