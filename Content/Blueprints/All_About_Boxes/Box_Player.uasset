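; Collectible box that drops from a head location to a drop point and can then be picked up by a Hamster.
; On BeginPlay it picks a random mesh and material, which RepNotify functions apply to the static mesh.
; BoxDrop lerps the actor along a timeline and makes it takeable when finished.
; A Hamster overlap then increases that character's scale and box count once and destroys the box.
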(event `self.ReceiveBeginPlay`
  ;[1 1 1] Меш и материал
  (`self.BoxSetMatAndMesh`))

(event `BoxSetMatAndMesh`
  ;[1 1 1] Меш и материал
  (set `self.Mesh` (`|GetArrayItem` (`self.BoxMeshes`) (`KismetMathLibrary.RandomInteger` 2)))
  (set `self.Mat` (`|GetArrayItem` (`self.BoxMaterials`) (`KismetMathLibrary.RandomInteger` 12))))

(event `BoxDrop`
  (bind (_direction _newtrack_0) (`Timeline|Timeline_0` :!via `PlayFromStart`)
    (:`Update`
      (`self.K2_SetActorLocation` (`KismetMathLibrary.VLerp` (`self.HeadLocation`) (`self.DropPointLocation`) _newtrack_0)))
    (:`Finished`
      (set `self.Tackabl?` true))))

(event `self.Box.OnComponentBeginOverlap`
  (params (OverlappedComponent :type "PrimitiveComponent Object Reference") (OtherActor :type "Actor Object Reference") (OtherComp :type "PrimitiveComponent Object Reference") (OtherBodyIndex :type Integer) (bFromSweep :type Boolean) (SweepResult :type "HitResult Structure (by ref)"))
  (bind _character_ref (`self.Character_Ref`))
  (if (`self.Tackabl?`)
    (bind _ashamster (cast `/Game/Character/Humster/Hamster` OtherActor))
    (bind _output_get (set `self.Character_Ref` _ashamster))
    (`/Engine/EditorBlueprintResources/StandardMacros.DoOnce` false
      (:`Completed`
        (`/Game/Character/Humster/Hamster.CalculateScale` _output_get "Inc" 1)
        ;[1 1 1 0] Добавление числа в общее количество коробок
        (set `/Game/Character/Humster/Hamster.Boxes_In_Character` (+ (`/Game/Character/Humster/Hamster.Boxes_In_Character` _character_ref) 1) _character_ref)
        (`self.K2_DestroyActor`)))))

(fn `OnRep_Mat`
  (`PrimitiveComponent.SetMaterial` (`self.StaticMesh`) 0 (`self.Mat`)))

(fn `OnRep_Mesh`
  (`StaticMeshComponent.SetStaticMesh` (`self.StaticMesh`) (`self.Mesh`)))

(fn `UserConstructionScript`)