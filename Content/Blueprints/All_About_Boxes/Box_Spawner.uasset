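; Spawner actor that keeps the level's Box_Spawn_Point actors stocked with Box_World pickups on a repeating timer.
; Shortly after BeginPlay, server events gather all spawn points, run a first pass and start the looping timer.
; Each pass collects points with no box and nobody standing on them, spawns boxes there from the array's end, then links each box to its point and marks it occupied.
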(event `self.ReceiveBeginPlay`
  ;[1 0.07286 0.08281] Begin Play
  (`KismetSystemLibrary.Delay` 0.2)
  (`self.Server_StartSpawnBoxes`))

(event `Server_StartSpawnBoxes`
  ;[1 1 1] Найти все возможные точки спавна коробок на карте, записать в массив и запустить спавн
  (bind _outactors (`GameplayStatics.GetAllActorsOfClass` "/Game/Blueprints/All_About_Boxes/Box_Spawn_Point.Box_Spawn_Point_C"))
  (bind _output_get (set `self.Box_Spawn_Points` _outactors))
  (`KismetArrayLibrary.Array_Append` _output_get (`self.Able_Points`))
  (`self.Server_SpawnBoxesInLevel`))

(event `Server_SpawnBoxesInLevel`
  ;[1 1 1] Запустить спавн коробок на сервере и клиентах
  (`self.Spawn_Boxes_On_Points`)
  (`KismetSystemLibrary.K2_SetTimerDelegate` (delegate `Spawn_Boxes_On_Points`) (`self.Boxs_Spawn_Delay`) true))

(event `Spawn_Boxes_On_Points`
  (bind _able_points (`self.Able_Points`))
  ;[1 1 1] Если на выбранной точке нет коробки и на ней не стоит игрок, то добавить точку в массив доступных
  (`KismetArrayLibrary.Array_Clear` (`self.Able_Points`))
  (for _array_element (`self.Box_Spawn_Points`)
    (bind _output_get (set `self.Spawn_Point` _array_element))
    (if (`/Game/Blueprints/All_About_Boxes/Box_Spawn_Point.Box_Already_On_Point` _output_get)
      _
      (elif (not (`/Game/Blueprints/All_About_Boxes/Box_Spawn_Point.Someone_On_Me` _output_get))
        (`KismetArrayLibrary.Array_Add` (`self.Able_Points`) (`self.Spawn_Point`)))))
  ;[1 1 1] Все ли точки заняты?
  (if (not (<= (`KismetArrayLibrary.Array_Length` (`self.Able_Points`)) 0))
    ;[1 1 1] Спавн коробок на доступных точках
    (for _ (range (+ (`KismetMathLibrary.Min` (`KismetArrayLibrary.Array_Length` (`self.Able_Points`)) (`KismetArrayLibrary.Array_LastIndex` (`self.Box_Spawn_Points`))) 1))
      (bind _output_get_2 (set `self.Current_Point` (`KismetArrayLibrary.Array_LastIndex` _able_points)))
      (bind _output_get_3 (set `self.TakedSpawnPoint` (`|GetArrayItem` _able_points _output_get_2)))
      (if (not (`/Game/Blueprints/All_About_Boxes/Box_Spawn_Point.Someone_On_Me` _output_get_3))
        (bind _returnvalue (`|SpawnActorFromClass` "/Game/Blueprints/All_About_Boxes/Box_World.Box_World_C" (`KismetMathLibrary.MakeTransform` (`self.K2_GetActorLocation` (`self.TakedSpawnPoint`))) "Undefined" "OverrideRootScale" null null))
        (bind _output_get_4 (set `/Game/Blueprints/All_About_Boxes/Box_World.My_Spawn_Point` (`self.TakedSpawnPoint`) _returnvalue))
        (set `/Game/Blueprints/All_About_Boxes/Box_Spawn_Point.Box_Already_On_Point` true _output_get_4)
        (`KismetArrayLibrary.Array_Remove` (`self.Able_Points`) (`self.Current_Point`))))))

(fn `UserConstructionScript`)