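; Bear trap (kapkan) actor disguised as a box, which springs on a Hamster that touches it.
; BeginPlay picks a random mesh and material, applied through OnRep functions, and BoxDrop runs a timeline that moves it to the drop point and arms it.
; On overlap when armed, it calls KapkanHit, swaps the box for the snapping trap, attaches to the hamster's Kapkan_Socket and destroys itself after a delay.
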(event `self.ReceiveBeginPlay`
  ;[1 1 1] Меш и материал
  (`self.BoxSetMatAndMesh`))

(event `BoxSetMatAndMesh`
  ;[1 1 1] Меш и материал
  (set `self.Mesh` (`|GetArrayItem` (`self.BoxMeshes`) (`KismetMathLibrary.RandomInteger` 2)))
  (set `self.Mat` (`|GetArrayItem` (`self.BoxMaterials`) (`KismetMathLibrary.RandomInteger` 12))))

(event `FAW`
  (params (Target :type "Character Object Reference"))
  (`self.K2_AttachToComponent` (`/Game/Character/Humster/Hamster.SkeletalMesh` (stale `self.Box.OnComponentBeginOverlap` _ashamster)) "Kapkan_Socket" "SnapToTarget" "SnapToTarget" "SnapToTarget" :!label _label)
  (`KismetSystemLibrary.Delay` 5.0)
  (`self.K2_DestroyActor`))

(event `self.Box.OnComponentBeginOverlap`
  (params (OverlappedComponent :type "PrimitiveComponent Object Reference") (OtherActor :type "Actor Object Reference") (OtherComp :type "PrimitiveComponent Object Reference") (OtherBodyIndex :type Integer) (bFromSweep :type Boolean) (SweepResult :type "HitResult Structure (by ref)"))
  (bind _ashamster (cast `/Game/Character/Humster/Hamster` OtherActor))
  (set `self.Character_Ref` _ashamster)
  (if (`self.Tackabl?`)
    (`KismetSystemLibrary.Delay` 0.1)
    (`/Game/Character/Humster/Hamster.Kapkan_Hit` _ashamster)
    (`SceneComponent.SetVisibility` (`self.Trap`) true false)
    (`SceneComponent.SetVisibility` (`self.StaticMesh`) false false)
    (`SkeletalMeshComponent.PlayAnimation` (`self.Trap`) "/Game/Blueprints/All_About_Boxes/BearTrap_SnapShut_Anim.BearTrap_SnapShut_Anim" false)
    (goto _label)))

(event `BoxDrop`
  (bind (_direction _newtrack_0) (`Timeline|Timeline_0` :!via `PlayFromStart`)
    (:`Update`
      (`self.K2_SetActorLocation` (`KismetMathLibrary.VLerp` (`self.HeadLocation`) (`self.DropPointLocation`) _newtrack_0)))
    (:`Finished`
      (set `self.Tackabl?` true))))

(fn `OnRep_Mat`
  (`PrimitiveComponent.SetMaterial` (`self.StaticMesh`) 0 (`self.Mat`)))

(fn `OnRep_Mesh`
  (`StaticMeshComponent.SetStaticMesh` (`self.StaticMesh`) (`self.Mesh`)))

(fn `UserConstructionScript`)