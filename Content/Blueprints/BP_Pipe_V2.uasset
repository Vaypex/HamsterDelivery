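; A spline-shaped pipe that carries a Hamster along its path when the Hamster overlaps the Enter component.
; The construction script tiles collidable spline meshes in sections sized by actor X scale, with tangents clamped to section length.
; It also adds an Exit box at the last section's end, which the event graph never uses.
; On overlap, GoPipe plays a timeline that sets the Hamster's location and rotation from the spline.
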(event `self.Enter.OnComponentBeginOverlap`
  (params (OverlappedComponent :type "PrimitiveComponent Object Reference") (OtherActor :type "Actor Object Reference") (OtherComp :type "PrimitiveComponent Object Reference") (OtherBodyIndex :type Integer) (bFromSweep :type Boolean) (SweepResult :type "HitResult Structure (by ref)"))
  (bind _ashamster (cast `/Game/Character/Humster/Hamster` OtherActor))
  (`self.GoPipe` _ashamster))

(event `GoPipe`
  (params (`Humster Actor` :type "Actor Object Reference"))
  (bind _spline (`self.Spline`))
  (bind (_direction _newtrack_1) (`Timeline|Timeline_0` :!via `PlayFromStart`)
    (:`Update`
      (`self.K2_SetActorTransform` `Humster Actor` (`KismetMathLibrary.MakeTransform` (`SplineComponent.GetLocationAtTime` _spline _newtrack_1 "World" false) (`SplineComponent.GetRotationAtTime` _spline _newtrack_1 "World" false)) false false))))

(fn `UserConstructionScript`
  (bind _returnvalue_x (`KismetMathLibrary.BreakVector` (`self.GetActorScale3D`)))
  (bind _spline (`self.Spline`))
  (bind _spline_2 (`self.Spline`))
  (set `self.Section Lenght` (* _returnvalue_x 100.0))
  (for _index (range (`KismetMathLibrary.FTrunc` (/ (`SplineComponent.GetSplineLength` (`self.Spline`)) (`self.Section Lenght`))))
    (bind _returnvalue (`AddComponent|NODE_AddSplineMeshComponent-0` :`RelativeTransform` (`KismetMathLibrary.MakeTransform` (0.0 0.0 0.0) (struct) (1.0 1.0 1.0))))
    (`SplineMeshComponent.SetForwardAxis` _returnvalue "X" true)
    (`PrimitiveComponent.SetCollisionEnabled` _returnvalue "QueryAndPhysics")
    (bind _returnvalue_2 (* _index (`self.Section Lenght`)))
    (bind _returnvalue_3 (* (+ _index 1) (`self.Section Lenght`)))
    (bind _returnvalue_4 (`SplineComponent.GetLocationAtDistanceAlongSpline` _spline _returnvalue_3 "Local"))
    (`SplineMeshComponent.SetStartAndEnd` _returnvalue (`SplineComponent.GetLocationAtDistanceAlongSpline` _spline_2 _returnvalue_2 "Local") (`KismetMathLibrary.ClampVectorSize` (`SplineComponent.GetTangentAtDistanceAlongSpline` _spline_2 _returnvalue_2 "Local") 0.0 (`self.Section Lenght`)) _returnvalue_4 (`KismetMathLibrary.ClampVectorSize` (`SplineComponent.GetTangentAtDistanceAlongSpline` _spline _returnvalue_3 "Local") 0.0 (`self.Section Lenght`)) true)
    (set `self.EndPos` _returnvalue_4))
  (bind _returnvalue_5 (`AddComponent|NODE_AddBoxComponent-2` :`RelativeTransform` (`KismetMathLibrary.MakeTransform` (`self.EndPos`))))
  (set `self.Exit` _returnvalue_5))