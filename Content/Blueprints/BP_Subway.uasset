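; BP_Subway is a teleport station that sends a Hamster entering its Box to the next subway station in the level.
; On BeginPlay each station gathers all BP_Subway actors, and an overlap picks the entry after itself, wrapping to the first.
; The Hamster moves to that station's Arrow transform.
; The Hamster's HatchTeleporting flag and a DoOnce, both cleared after a short delay, block immediate re-teleporting.
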(event `self.ReceiveBeginPlay`
  (if (not (`self.Set`))
    (`self.Server`)))

(event `Server`
  (set `self.Set` true)
  (bind _outactors (`GameplayStatics.GetAllActorsOfClass` "BP_Subway_C"))
  (bind _output_get (set `self.Out Actors` _outactors))
  (for _ _output_get
    _))

(event `self.Box.OnComponentBeginOverlap`
  (params (OverlappedComponent :type "PrimitiveComponent Object Reference") (OtherActor :type "Actor Object Reference") (OtherComp :type "PrimitiveComponent Object Reference") (OtherBodyIndex :type Integer) (bFromSweep :type Boolean) (SweepResult :type "HitResult Structure (by ref)"))
  (bind _arrow (`/Game/Blueprints/BP_Subway.Arrow` (`self.Station`)))
  (bind _ashamster (cast `/Game/Character/Humster/Hamster` OtherActor))
  (set `self.As Hamster` _ashamster)
  (if (not (`/Game/Character/Humster/Hamster.HatchTeleporting?` _ashamster))
    (set `/Game/Character/Humster/Hamster.HatchTeleporting?` true _ashamster)
    (`/Engine/EditorBlueprintResources/StandardMacros.DoOnce` false :!label _label
      (:`Completed`
        (if (== (`KismetArrayLibrary.Array_Find` (`self.Out Actors`) self) (- (`KismetArrayLibrary.Array_Length` (`self.Out Actors`)) 1))
          (set `self.Station` (`|GetArrayItem` (`self.Out Actors`)))
          (else
            (bind _output_get (set `self.Station` (`|GetArrayItem` (`self.Out Actors`) (+ (`KismetArrayLibrary.Array_Find` (`self.Out Actors`) self) 1))))
            (`KismetSystemLibrary.PrintString` (`KismetSystemLibrary.GetDisplayName` _output_get))))
        (`self.K2_SetActorLocationAndRotation` (`self.As Hamster`) (`SceneComponent.K2_GetComponentLocation` _arrow) (`SceneComponent.K2_GetComponentRotation` _arrow) false false)
        (`KismetSystemLibrary.Delay` 2.0)
        (set `/Game/Character/Humster/Hamster.HatchTeleporting?` false (`self.As Hamster`))
        (goto _label :!via `Reset`)))))

(fn `UserConstructionScript`)