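; BP_ManHole is a manhole that teleports an overlapping Hamster carrying 15 or fewer boxes toward other manholes.
; Sphere1 overlaps slide the cover open and closed through the OpenClose timeline, while Sphere triggers the teleport.
; The teleport launches the hamster upward, closes this cover, then clears HatchTeleporting after a delay.
; Destination X, Y and Z each roll their own random index, so coordinates can mix different holes.
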(event `self.ReceiveBeginPlay`
  (bind (_returnvalue_x _returnvalue_y _returnvalue_z) (`KismetMathLibrary.BreakVector` (`self.K2_GetActorLocation`)))
  (`KismetSystemLibrary.Delay` 0.2)
  (bind _outactors (`GameplayStatics.GetAllActorsOfClass` "BP_ManHole_C"))
  (bind _output_get (set `self.All Holes` _outactors))
  (`KismetArrayLibrary.Array_RemoveItem` _output_get self)
  (set `self.Open_Location` (`KismetMathLibrary.MakeVector` (+ _returnvalue_x 100.0) _returnvalue_y _returnvalue_z))
  (set `self.Close_Location` (`self.K2_GetActorLocation`)))

(event `self.Sphere.OnComponentBeginOverlap`
  (params (OverlappedComponent :type "PrimitiveComponent Object Reference") (OtherActor :type "Actor Object Reference") (OtherComp :type "PrimitiveComponent Object Reference") (OtherBodyIndex :type Integer) (bFromSweep :type Boolean) (SweepResult :type "HitResult Structure (by ref)"))
  (bind _ashamster (cast `/Game/Character/Humster/Hamster` OtherActor))
  (if (not (`/Game/Character/Humster/Hamster.HatchTeleporting?` _ashamster))
    (bind _output_get (set `self.As Hamster` _ashamster))
    (set `/Game/Character/Humster/Hamster.HatchTeleporting?` true _output_get)
    (if (<= (`/Game/Character/Humster/Hamster.Boxes_In_Character` _output_get) 15)
      (`self.ManholeLogic`))))

(event `ManholeLogic`
  (bind _returnvalue (`KismetArrayLibrary.Array_Length` (`self.All Holes`)))
  (bind _output (`|GetArrayItem` (`self.All Holes`) (`KismetMathLibrary.RandomIntegerInRange` 0 (- _returnvalue 1))))
  (bind (_returnvalue_x _returnvalue_y _returnvalue_z) (`KismetMathLibrary.BreakVector` (`self.K2_GetActorLocation` _output)))
  (bind (_returnvalue_x_2 _returnvalue_y_2) (`KismetMathLibrary.BreakVector` (`self.K2_GetActorLocation` _output)))
  (`/Engine/EditorBlueprintResources/StandardMacros.DoOnce` false :!label _label
    (:`Completed`
      (`KismetSystemLibrary.PrintString` (`KismetStringLibrary.Conv_IntToString` _returnvalue))
      (`self.K2_SetActorLocation` (`self.As Hamster`) (`KismetMathLibrary.MakeVector` _returnvalue_x _returnvalue_y (+ _returnvalue_z 50.0)) false false)
      (`|ExecutionSequence`
        (:`then_0`
          (`Character.LaunchCharacter` (`self.As Hamster`) (`KismetMathLibrary.MakeVector` (`KismetMathLibrary.RandomFloatInRange` (+ _returnvalue_x_2 50.0) 50.0) (`KismetMathLibrary.RandomFloatInRange` (+ _returnvalue_y_2 1.0) 50.0) 500.0) false false)
          (bind (_direction _newtrack_0) (`Timeline|Timeline_Manhole` :!via `PlayFromStart`)
            (:`Update`
              (`SceneComponent.K2_SetWorldLocation` (`self.StaticMesh`) (`KismetMathLibrary.VLerp` (`self.Open_Location`) (`self.Close_Location`) _newtrack_0) false false))
            (:`Finished`
              (`KismetSystemLibrary.Delay` 2.0)
              (set `/Game/Character/Humster/Hamster.HatchTeleporting?` false (`self.As Hamster`))
              (goto _label :!via `Reset`))))))))

(event `self.Sphere1.OnComponentBeginOverlap`
  (params (OverlappedComponent :type "PrimitiveComponent Object Reference") (OtherActor :type "Actor Object Reference") (OtherComp :type "PrimitiveComponent Object Reference") (OtherBodyIndex :type Integer) (bFromSweep :type Boolean) (SweepResult :type "HitResult Structure (by ref)"))
  (cast `/Game/Character/Humster/Hamster` OtherActor)
  (`|ExecutionSequence`
    (:`then_0`
      (`/Engine/EditorBlueprintResources/StandardMacros.DoOnce` false :!label _label_2
        (:`Completed`
          (set `self.CanJumpInHole?` true)
          (bind (_direction _newtrack_0) (`Timeline|Open/Close` :!via `PlayFromStart` :!label _label_3)
            (:`Update`
              (`SceneComponent.K2_SetWorldLocation` (`self.StaticMesh`) (`KismetMathLibrary.VLerp` (`self.Close_Location`) (`self.Open_Location`) _newtrack_0) false false))))))
    (:`then_1`
      (goto _label_4 :!via `Reset`))))

(event `self.Sphere1.OnComponentEndOverlap`
  (params (OverlappedComponent :type "PrimitiveComponent Object Reference") (OtherActor :type "Actor Object Reference") (OtherComp :type "PrimitiveComponent Object Reference") (OtherBodyIndex :type Integer))
  (cast `/Game/Character/Humster/Hamster` OtherActor)
  (`|ExecutionSequence`
    (:`then_0`
      (`/Engine/EditorBlueprintResources/StandardMacros.DoOnce` false :!label _label_4
        (:`Completed`
          (set `self.CanJumpInHole?` false)
          (goto _label_3 :!via `Reverse`))))
    (:`then_1`
      (goto _label_2 :!via `Reset`))))

(fn `UserConstructionScript`)