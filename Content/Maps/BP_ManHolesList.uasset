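; BP_ManHolesList is a level manager that links every manhole actor in the map to the others.
; On BeginPlay it gathers all BP_ManHole actors, stores them in AllManHoles and prints the count.
; It then appends the full list, including each manhole itself, to every manhole's AllHoles array.
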(event `self.ReceiveBeginPlay`
  (`self.FindHoles`))

(event `FindHoles`
  (bind _outactors (`GameplayStatics.GetAllActorsOfClass` "/Game/Maps/BP_ManHole.BP_ManHole_C"))
  (bind _output_get (set `self.AllManHoles` _outactors))
  (`KismetSystemLibrary.PrintString` (`KismetStringLibrary.Conv_IntToString` (`KismetArrayLibrary.Array_Length` _output_get)))
  (for _array_element _output_get
    (`KismetArrayLibrary.Array_Append` (`/Game/Maps/BP_ManHole.All Holes` _array_element) (`self.AllManHoles`))))

(fn `UserConstructionScript`)