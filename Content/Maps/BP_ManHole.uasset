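; Manhole actor that teleports an overlapping Hamster carrying no more than a set number of boxes to another manhole.
; It removes itself from AllHoles, picks a random remaining entry, places the hamster just above it and launches it upward.
; A timeline then offsets this manhole's mesh along X, and a DoOnce blocks retriggering until a short delay after the timeline finishes.
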(event `self.ReceiveBeginPlay`)

(event `self.Sphere.OnComponentBeginOverlap`
  (params (OverlappedComponent :type "PrimitiveComponent Object Reference") (OtherActor :type "Actor Object Reference") (OtherComp :type "PrimitiveComponent Object Reference") (OtherBodyIndex :type Integer) (bFromSweep :type Boolean) (SweepResult :type "HitResult Structure (by ref)"))
  (bind _ashamster (cast `/Game/Character/Humster/Hamster` OtherActor))
  (bind _output_get (set `self.As Hamster` _ashamster))
  (if (<= (`/Game/Character/Humster/Hamster.Boxes_In_Character` _output_get) 20)
    (`self.ManholeLogic`)))

(event `ManholeLogic`
  (bind (_deflocation_x _deflocation_y _deflocation_z) (`KismetMathLibrary.BreakVector` (`self.DefLocation`)))
  (bind _returnvalue (`KismetArrayLibrary.Array_Length` (`self.All Holes`)))
  (bind (_returnvalue_x _returnvalue_y _returnvalue_z) (`KismetMathLibrary.BreakVector` (`self.K2_GetActorLocation` (`|GetArrayItem` (`self.All Holes`) (`KismetMathLibrary.RandomIntegerInRange` 0 (- _returnvalue 1))))))
  (`/Engine/EditorBlueprintResources/StandardMacros.DoOnce` false :!label _label
    (:`Completed`
      (`KismetArrayLibrary.Array_RemoveItem` (`self.All Holes`) self)
      (`KismetSystemLibrary.PrintString` (`KismetStringLibrary.Conv_IntToString` _returnvalue))
      (`self.K2_SetActorLocation` (`self.As Hamster`) (`KismetMathLibrary.MakeVector` _returnvalue_x _returnvalue_y (+ _returnvalue_z 50.0)) false false)
      (`Character.LaunchCharacter` (`self.As Hamster`) (0.0 0.0 1000.0) false false)
      (bind (_direction _newtrack_0) (`Timeline|Timeline_Manhole` :!via `PlayFromStart`)
        (:`Update`
          (`SceneComponent.K2_SetRelativeLocation` (`self.StaticMesh`) (`KismetMathLibrary.VLerp` (`self.DefLocation`) (`KismetMathLibrary.MakeVector` (+ _deflocation_x 50.0) _deflocation_y _deflocation_z) _newtrack_0) false false))
        (:`Finished`
          (`KismetSystemLibrary.Delay` 3.0)
          (goto _label :!via `Reset`))))))

(fn `UserConstructionScript`)